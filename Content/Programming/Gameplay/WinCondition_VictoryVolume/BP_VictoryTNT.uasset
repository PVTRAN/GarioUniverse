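; BP_VictoryTNT is a victory TNT actor that sets off the level's destruction and reports a win or loss.
; Its box overlap toggles a prompt widget and the player's ExplosionCamReady flag.
; Explode reattaches the player's follow camera to NewCameraLocation and explodes every DestructableActors entry.
; It then sends the next level name and result to the game mode, losing only when Timer is set and no safe point was reached.
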(event `self.ReceiveBeginPlay`
  (`SceneComponent.SetVisibility` (`self.Widget`) false false)
  (bind _asbp_third_person_character (cast `/Game/Unreal_Asset/ThirdPerson/Blueprints/BP_ThirdPersonCharacter` (`GameplayStatics.GetPlayerCharacter` 0)))
  (set `self.Player` _asbp_third_person_character))

(event `self.Box.OnComponentBeginOverlap`
  (params (OverlappedComponent :type "PrimitiveComponent Object Reference") (OtherActor :type "Actor Object Reference") (OtherComp :type "PrimitiveComponent Object Reference") (OtherBodyIndex :type Integer) (bFromSweep :type Boolean) (SweepResult :type "HitResult Structure (by ref)"))
  (if (== OtherActor (`GameplayStatics.GetPlayerCharacter` 0))
    (`SceneComponent.SetVisibility` (`self.Widget`) true false)
    (set `/Game/Unreal_Asset/ThirdPerson/Blueprints/BP_ThirdPersonCharacter.ExplosionCamReady?` true (`self.Player`))))

(event `self.Box.OnComponentEndOverlap`
  (params (OverlappedComponent :type "PrimitiveComponent Object Reference") (OtherActor :type "Actor Object Reference") (OtherComp :type "PrimitiveComponent Object Reference") (OtherBodyIndex :type Integer))
  (if (== OtherActor (`GameplayStatics.GetPlayerCharacter` 0))
    (`SceneComponent.SetVisibility` (`self.Widget`) false false)
    (set `/Game/Unreal_Asset/ThirdPerson/Blueprints/BP_ThirdPersonCharacter.ExplosionCamReady?` false (`self.Player`))))

(fn `Explode`
  (`SceneComponent.K2_AttachToComponent` (`/Game/Unreal_Asset/ThirdPerson/Blueprints/BP_ThirdPersonCharacter.FollowCamera` (`self.Player`)) (`Actor.RootComponent` (`self.NewCameraLocation`)) "None" "KeepRelative" "KeepRelative" "KeepRelative" true)
  (for _array_element (`self.DestructableActors`)
    (`/Game/Programming/Gameplay/WinCondition_VictoryVolume/BP_DestructableActor.explode` _array_element))
  (if (`self.Timer?`)
    (if (`/Game/Unreal_Asset/ThirdPerson/Blueprints/BP_ThirdPersonCharacter.ReachedSafePoint?` (`self.Player`))
      (message `/Game/BPI_Gamemode.SetTimeDilation` (`GameplayStatics.GetGameMode`) (`self.Name Of Next Level`) true)
      (else
        (message `/Game/BPI_Gamemode.SetTimeDilation` (`GameplayStatics.GetGameMode`) (`self.Name Of Next Level`) false)))
    (else
      (message `/Game/BPI_Gamemode.SetTimeDilation` (`GameplayStatics.GetGameMode`) (`self.Name Of Next Level`) true))))

(fn `UserConstructionScript`)