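; BP_DeathField is a boundary actor that costs the player a life for staying outside its YouAreDead volume.
; Leaving the volume sets DeathTimerActive and starts a three-second Delay, while re-entering clears the flag.
; If the flag is still set afterwards, it decrements Lives on the player's health component and calls ResetPlayerMessage on the game mode.
; Tick prints a debug warning while the flag is set.
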(event `self.ReceiveBeginPlay`
  (bind _asbp_third_person_character (cast `/Game/Unreal_Asset/ThirdPerson/Blueprints/BP_ThirdPersonCharacter` (`GameplayStatics.GetPlayerCharacter` 0)))
  (set `self.Player` _asbp_third_person_character))

(event `self.ReceiveTick`
  (params (DeltaSeconds :type "Float (single-precision)"))
  (if (`self.DeathTimerActive`)
    (`KismetSystemLibrary.PrintString` "player gonna dieeeeeee" true true (struct :`G` 0.66 :`B` 1.0 :`A` 1.0) 0.1)))

(event `self.YouAreDead!.OnComponentEndOverlap`
  (params (OverlappedComponent :type "PrimitiveComponent Object Reference") (OtherActor :type "Actor Object Reference") (OtherComp :type "PrimitiveComponent Object Reference") (OtherBodyIndex :type Integer))
  (bind _bpc_health_component (`/Game/Unreal_Asset/ThirdPerson/Blueprints/BP_ThirdPersonCharacter.BPC_Health_Component` (`self.Player`)))
  (if (== OtherActor (`GameplayStatics.GetPlayerCharacter` 0))
    (set `self.DeathTimerActive` true)
    (`KismetSystemLibrary.Delay` 3.0)
    (if (`self.DeathTimerActive`)
      (set `/Game/Programming/Character/BPC_Health_Component.Lives` (- (`/Game/Programming/Character/BPC_Health_Component.Lives` _bpc_health_component) 1.0) _bpc_health_component)
      (message `/Game/BPI_Gamemode.ResetPlayer` (`GameplayStatics.GetGameMode`)))))

(event `self.YouAreDead!.OnComponentBeginOverlap`
  (params (OverlappedComponent :type "PrimitiveComponent Object Reference") (OtherActor :type "Actor Object Reference") (OtherComp :type "PrimitiveComponent Object Reference") (OtherBodyIndex :type Integer) (bFromSweep :type Boolean) (SweepResult :type "HitResult Structure (by ref)"))
  (if (== OtherActor (`GameplayStatics.GetPlayerCharacter` 0))
    (set `self.DeathTimerActive` false)))

(fn `UserConstructionScript`)