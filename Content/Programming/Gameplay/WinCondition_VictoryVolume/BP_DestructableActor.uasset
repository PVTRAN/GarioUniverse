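; BP_DestructableActor is a destructible prop that swaps a static mesh for a Geometry Collection when it explodes.
; The Geometry Collection stays inactive on BeginPlay, with physics, tick and collision off to keep it dormant until needed.
; Explode destroys the mesh, enables and crumbles the collection, sets a gravity state on its GravityVolume and fires a RadialForce impulse.
; The actor then removes itself after a short lifespan.
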(event `self.ReceiveBeginPlay`
  (bind _geometrycollection (`self.GeometryCollection`))
  (bind _geometrycollection_2 (`self.GeometryCollection`))
  (`ActorComponent.SetActive` _geometrycollection_2 false false)
  (`PrimitiveComponent.SetSimulatePhysics` _geometrycollection_2 false)
  (`ActorComponent.SetComponentTickEnabled` _geometrycollection false)
  (`PrimitiveComponent.SetCollisionEnabled` _geometrycollection "NoCollision"))

(fn `explode`
  (bind _geometrycollection (`self.GeometryCollection`))
  (`PrimitiveComponent.SetCollisionEnabled` (`self.GeometryCollection`) "QueryAndPhysics")
  (`ActorComponent.K2_DestroyComponent` (`self.StaticMesh`))
  (`PrimitiveComponent.SetSimulatePhysics` _geometrycollection true)
  (`ActorComponent.SetActive` _geometrycollection true false)
  (`GeometryCollectionComponent.SetEnableDamageFromCollision` _geometrycollection true)
  (`ActorComponent.SetComponentTickEnabled` (`self.GeometryCollection`) true)
  (`GeometryCollectionComponent.CrumbleCluster` _geometrycollection 0)
  (message `/Game/Programming/Gravity/BPI_Gravity_Object.SetVolumeGravityState` (`self.GravityVolume`) "NewEnumerator2")
  (`RadialForceComponent.FireImpulse` (`self.RadialForce`))
  (`self.SetLifeSpan` 2.0))

(fn `UserConstructionScript`)