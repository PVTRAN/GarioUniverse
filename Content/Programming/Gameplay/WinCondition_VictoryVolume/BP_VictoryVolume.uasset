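; BP_VictoryVolume is a trigger actor that marks the safe point for the win condition.
; On BeginPlay it caches the player's BP_ThirdPersonCharacter.
; When that character overlaps the VolumeForVictory component, a DoOnce flags the character's ReachedSafePoint and calls Explode on its TNT reference.
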(event `self.ReceiveBeginPlay`
  (bind _asbp_third_person_character (cast `/Game/Unreal_Asset/ThirdPerson/Blueprints/BP_ThirdPersonCharacter` (`GameplayStatics.GetPlayerCharacter` 0)))
  (set `self.Player` _asbp_third_person_character))

(event `self.VolumeForVictory.OnComponentBeginOverlap`
  (params (OverlappedComponent :type "PrimitiveComponent Object Reference") (OtherActor :type "Actor Object Reference") (OtherComp :type "PrimitiveComponent Object Reference") (OtherBodyIndex :type Integer) (bFromSweep :type Boolean) (SweepResult :type "HitResult Structure (by ref)"))
  (bind _player (`self.Player`))
  (if (== OtherActor _player)
    (`/Engine/EditorBlueprintResources/StandardMacros.DoOnce` false
      (:`Completed`
        (set `/Game/Unreal_Asset/ThirdPerson/Blueprints/BP_ThirdPersonCharacter.ReachedSafePoint?` true _player)
        (`/Game/Programming/Gameplay/WinCondition_VictoryVolume/BP_VictoryTNT.Explode` (`/Game/Unreal_Asset/ThirdPerson/Blueprints/BP_ThirdPersonCharacter.TNTRef` _player))))))

(fn `UserConstructionScript`)