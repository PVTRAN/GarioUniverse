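; Non-homing asteroid hazard that flies at the spot where the player stood at BeginPlay and damages the player on contact.
; A Timeline moves the Sphere toward that saved mesh location with VInterpToConstant plus a Movement track offset, using delta time cached on Tick.
; Sphere1 overlap with the player applies environmental damage and destroys the actor, which also self-destructs when the Timeline finishes.
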(event `self.ReceiveBeginPlay`
  (bind _delta_seconds (`self.Delta Seconds`))
  ;[1 1 1] Tracks Movement of Player and Moves With Them
  (set `self.PlayerLocation` (`SceneComponent.K2_GetComponentLocation` (`Character.Mesh` (`GameplayStatics.GetPlayerCharacter` 0))))
  (bind (_direction _movement) (`Timeline|Timeline`)
    (:`Update`
      (`SceneComponent.K2_SetWorldLocation` (`self.Sphere`) (+ _movement (`KismetMathLibrary.VInterpTo_Constant` (`SceneComponent.K2_GetComponentLocation` (`self.Sphere`)) (`self.PlayerLocation`) _delta_seconds (+ _delta_seconds 3000.0))) false false))
    (:`Finished`
      (`self.K2_DestroyActor`))))

(event `self.ReceiveTick`
  (params (DeltaSeconds :type "Float (single-precision)"))
  ;[1 1 1] Tracks Movement of Player and Moves With Them
  (set `self.Delta Seconds` DeltaSeconds))

(event `self.Sphere1.OnComponentBeginOverlap`
  (params (OverlappedComponent :type "PrimitiveComponent Object Reference") (OtherActor :type "Actor Object Reference") (OtherComp :type "PrimitiveComponent Object Reference") (OtherBodyIndex :type Integer) (bFromSweep :type Boolean) (SweepResult :type "HitResult Structure (by ref)"))
  (bind _returnvalue (`GameplayStatics.GetPlayerCharacter` 0))
  ;[1 1 1] Applies Damage to Player
  (if (== OtherActor _returnvalue)
    (`GameplayStatics.ApplyDamage` _returnvalue (`self.Base Damage`) null self "/Engine/EngineDamageTypes/DmgTypeBP_Environmental.DmgTypeBP_Environmental_C")
    (`self.K2_DestroyActor`)))

(fn `UserConstructionScript`)