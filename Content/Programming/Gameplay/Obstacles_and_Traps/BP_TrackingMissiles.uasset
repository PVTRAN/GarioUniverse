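; BP_TrackingMissiles is a trap projectile that homes in on the first player's character.
; On BeginPlay a timeline moves its Sphere toward a point just above the player's mesh using VInterpToConstant, adding the timeline's Movement value as an offset.
; Tick only caches DeltaSeconds for that interpolation, and the actor destroys itself when the timeline finishes.
; The movement does not sweep, and the graph contains no hit or damage logic.
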(event `self.ReceiveBeginPlay`
  (bind _delta_seconds (`self.Delta Seconds`))
  (bind (_direction _movement) (`Timeline|Timeline`)
    (:`Update`
      (`SceneComponent.K2_SetWorldLocation` (`self.Sphere`) (+ _movement (`KismetMathLibrary.VInterpTo_Constant` (`SceneComponent.K2_GetComponentLocation` (`self.Sphere`)) (+ (`SceneComponent.K2_GetComponentLocation` (`Character.Mesh` (`GameplayStatics.GetPlayerCharacter` 0))) (0.0 0.0 100.0)) _delta_seconds (+ _delta_seconds 1000.0))) false false))
    (:`Finished`
      (`self.K2_DestroyActor`))))

(event `self.ReceiveTick`
  (params (DeltaSeconds :type "Float (single-precision)"))
  (set `self.Delta Seconds` DeltaSeconds))

(fn `UserConstructionScript`)