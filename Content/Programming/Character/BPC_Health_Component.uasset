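; Health component for characters that tracks current health and reacts to incoming damage.
; On BeginPlay it fills health to the maximum, and its damage event subtracts the received amount and prints the remaining value.
; When health drops to zero or below, it tells the GameMode to show the player death message, then immediately resets health to maximum.
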(event `self.ReceiveBeginPlay`
  (`self.SetMaxHealth`))

(event `Recieve Damage`
  (params (`recive damage` :type "Float (double-precision)"))
  ;[1 1 1] Damage Health
  (set `self.RecievedDamage` `recive damage`)
  (if (> (`self.Health`) 0.0)
    (bind _output_get (set `self.Health` (- (`self.Health`) (`self.RecievedDamage`))))
    (if (<= _output_get 0.0)
      (`KismetSystemLibrary.PrintString` "Im Dead")
      (message `/Game/BPI_Gamemode.Player Death` (`GameplayStatics.GetGameMode`))
      (`self.SetMaxHealth`)
      (else
        ;;[0 0 0] This will display remaining health
        (`KismetSystemLibrary.PrintString` (`KismetStringLibrary.Conv_DoubleToString` _output_get))))
    (else
      (`KismetSystemLibrary.PrintString` "already dead"))))

(fn `SetMaxHealth`
  (bind _output_get (set `self.Health` (`self.Max Health`)))
  (`KismetSystemLibrary.PrintString` (`KismetStringLibrary.Conv_DoubleToString` _output_get)))