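; BP_AlienMissle is an alien homing missile projectile that seeks the player character and explodes on hit or after a seven-second fuse.
; BeginPlay points ProjectileMovement's homing at the player's root component.
; Both triggers share one detonation path: explosion effect and sound, radial damage sized by the RadialForce radius, two impulses, then destruction.
; Hit also prints the struck actor's name, and the damage branch is hardwired true.
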(event `self.ReceiveBeginPlay`
  (bind _returnvalue (`self.K2_GetActorLocation`))
  (bind _returnvalue_2 (`GameplayStatics.GetPlayerCharacter` 0))
  (set `self.Homing target` _returnvalue_2)
  (set `ProjectileMovementComponent.HomingTargetComponent` (`Actor.RootComponent` _returnvalue_2) (`self.ProjectileMovement`))
  (set `ProjectileMovementComponent.bIsHomingProjectile` true (`self.ProjectileMovement`))
  (`KismetSystemLibrary.Delay` 7.0)
  (`GameplayStatics.SpawnEmitterAtLocation` "/Game/StarterContent/Particles/P_Explosion.P_Explosion" (`self.K2_GetActorLocation`) :!label _label)
  (`RadialForceComponent.FireImpulse` (`self.RadialForce`))
  (`GameplayStatics.PlaySoundAtLocation` "/Game/Audio/SFX/1S_TNT_Explosion.1S_TNT_Explosion" _returnvalue (struct) 1.0 1.0 0.0 null null null null)
  (if true
    (`GameplayStatics.ApplyRadialDamage` :`BaseDamage` 75.0 :`Origin` _returnvalue :`DamageRadius` (`RadialForceComponent.Radius` (`self.RadialForce`)) :`DamageCauser` null :`InstigatedByController` null :`DamagePreventionChannel` "ECC_GameTraceChannel1")
    (`RadialForceComponent.FireImpulse` (`self.RadialForce`))
    (`self.K2_DestroyActor`)
    (else
      (`self.K2_DestroyActor`))))

(event `self.ReceiveHit`
  (params (MyComp :type "PrimitiveComponent Object Reference") (Other :type "Actor Object Reference") (OtherComp :type "PrimitiveComponent Object Reference") (bSelfMoved :type Boolean) (HitLocation :type "Vector Structure") (HitNormal :type "Vector Structure") (NormalImpulse :type "Vector Structure") (Hit :type "HitResult Structure (by ref)"))
  (`KismetSystemLibrary.PrintString` (`KismetSystemLibrary.GetDisplayName` Other))
  (goto _label))

(fn `UserConstructionScript`)