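; BP_AlienBlackHole is a homing projectile that chases the player character and explodes after a seven-second delay or on hit.
; On BeginPlay it points ProjectileMovement at the player's root component.
; Both triggers share one detonation path that spawns an explosion effect and sound, fires the RadialForce impulse twice, then destroys the actor.
; A radial damage node exists but is never reached, so the blast only applies force.
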(event `self.ReceiveBeginPlay`
  (bind _returnvalue (`GameplayStatics.GetPlayerCharacter` 0))
  (set `self.Homing target` _returnvalue)
  (set `ProjectileMovementComponent.HomingTargetComponent` (`Actor.RootComponent` _returnvalue) (`self.ProjectileMovement`))
  (set `ProjectileMovementComponent.bIsHomingProjectile` true (`self.ProjectileMovement`))
  (`KismetSystemLibrary.Delay` 7.0)
  (`GameplayStatics.SpawnEmitterAtLocation` "/Game/StarterContent/Particles/P_Explosion.P_Explosion" (`self.K2_GetActorLocation`) :!label _label)
  (`RadialForceComponent.FireImpulse` (`self.RadialForce`))
  (`GameplayStatics.PlaySoundAtLocation` "/Game/Audio/SFX/1S_TNT_Explosion.1S_TNT_Explosion" (`self.K2_GetActorLocation`) (struct) 1.0 1.0 0.0 null null null null)
  (if true
    (`RadialForceComponent.FireImpulse` (`self.RadialForce`))
    (`self.K2_DestroyActor`)
    (else
      (`self.K2_DestroyActor`))))

(event `self.ReceiveHit`
  (params (MyComp :type "PrimitiveComponent Object Reference") (Other :type "Actor Object Reference") (OtherComp :type "PrimitiveComponent Object Reference") (bSelfMoved :type Boolean) (HitLocation :type "Vector Structure") (HitNormal :type "Vector Structure") (NormalImpulse :type "Vector Structure") (Hit :type "HitResult Structure (by ref)"))
  (`KismetSystemLibrary.PrintString` (`KismetSystemLibrary.GetDisplayName` Other))
  (goto _label))

(fn `UserConstructionScript`)