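; Game instance for Cracker that owns the player's persistent audio settings.
; LoadAudioSettings async-loads the audio save slot once, or creates and saves a new BP_AudioSaveGame if loading fails.
; A successful load applies master, music and SFX volumes as class overrides on SCM_Cracker; the newly created save path skips this step.
; SaveAudioSettings writes the cached save object back to the slot asynchronously.
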(event `LoadAudioSettings`
  ;[0 0 0 1 36] Audio Load/Save Logic [JLP 5/18/24]
  ;;[0 1 1] Load Audio [JLP 5/19/24] - Added Check to see if we have already loaded the audio settings
  (`/Engine/EditorBlueprintResources/StandardMacros.IsValid` (`self.AudioSaveGame`)
    (:`Is Not Valid`
      (bind (_savegame _bsuccess) (`AsyncActionHandleSaveGame.AsyncLoadGameFromSlot` (`self.AudioSettingsSlotName`))
        (:`Completed`
          (if _bsuccess
            (bind _asbp_audio_save_game (cast `/Game/Programming/Save/BP_AudioSaveGame` _savegame))
            (set `self.AudioSaveGame` _asbp_audio_save_game)
            (`self.OnAudioSettingsLoaded`)
            (else
              (bind _returnvalue (`GameplayStatics.CreateSaveGameObject` "/Game/Programming/Save/BP_AudioSaveGame.BP_AudioSaveGame_C"))
              (set `self.AudioSaveGame` _returnvalue)
              (`self.SaveAudioSettings`))))))))

(event `OnAudioSettingsLoaded`
  ;[0 0 0 1 36] Audio Load/Save Logic [JLP 5/18/24]
  ;;[0 1 1] On Audio Settings Loaded [JLP 5/18/24]
  (`self.InitializeSoundVolumes`))

(event `SaveAudioSettings`
  ;[0 0 0 1 36] Audio Load/Save Logic [JLP 5/18/24]
  ;;[0 1 1] Save Audio [JLP 5/18/24]
  (`AsyncActionHandleSaveGame.AsyncSaveGameToSlot` (`self.AudioSaveGame`) (`self.AudioSettingsSlotName`)))

(fn `InitializeSoundVolumes`
  (bind (_mastervol _musicvol _fxvol) (break `/Game/Programming/Save/S_AudioSettings` (`/Game/Programming/Save/BP_AudioSaveGame.AudioSettings` (`self.AudioSaveGame`))))
  (`GameplayStatics.SetSoundMixClassOverride` "/Game/Audio/Sound_Classes/SCM_Cracker.SCM_Cracker" "/Game/Audio/Sound_Classes/SC_Master.SC_Master" _mastervol 1.0 0.0)
  (`GameplayStatics.SetSoundMixClassOverride` "/Game/Audio/Sound_Classes/SCM_Cracker.SCM_Cracker" "/Game/Audio/Sound_Classes/SC_Music.SC_Music" _musicvol 1.0 0.0)
  (`GameplayStatics.SetSoundMixClassOverride` "/Game/Audio/Sound_Classes/SCM_Cracker.SCM_Cracker" "/Game/Audio/Sound_Classes/SC_SFX.SC_SFX" _fxvol 1.0 0.0))