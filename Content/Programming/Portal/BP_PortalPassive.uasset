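; BP_PortalPassive is a one-way link that teleports the player to its assigned exit portal while preserving speed.
; On BeginPlay it caches the player and optionally attaches itself to a specified actor.
; When ready, an Entry overlap moves the player to the exit's transform, then launches them along its forward vector at their previous speed.
; A brief CanTeleport lockout on the player prevents immediate re-teleporting.
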(event `self.ReceiveBeginPlay`
  (bind _attached_to_this_actor (`self.Attached to this actor`))
  (bind _asbp_third_person_character (cast `/Game/Unreal_Asset/ThirdPerson/Blueprints/BP_ThirdPersonCharacter` (`GameplayStatics.GetPlayerCharacter` 0)))
  (set `self.Player` _asbp_third_person_character)
  (`/Engine/EditorBlueprintResources/StandardMacros.IsValid` _attached_to_this_actor
    (:`Is Valid`
      (`self.K2_AttachToActor` _attached_to_this_actor "None" "KeepWorld" "KeepRelative" "KeepWorld"))))

(event `self.Entry.OnComponentBeginOverlap`
  (params (OverlappedComponent :type "PrimitiveComponent Object Reference") (OtherActor :type "Actor Object Reference") (OtherComp :type "PrimitiveComponent Object Reference") (OtherBodyIndex :type Integer) (bFromSweep :type Boolean) (SweepResult :type "HitResult Structure (by ref)"))
  (bind _exitportalpassive (`self.ExitPortalPassive`))
  (if (`self.Ready?`)
    (if (== OtherActor (`GameplayStatics.GetPlayerCharacter` 0))
      (if (`/Game/Unreal_Asset/ThirdPerson/Blueprints/BP_ThirdPersonCharacter.CanTeleport?` (`self.Player`))
        (`/Engine/EditorBlueprintResources/StandardMacros.IsValid` _exitportalpassive
          (:`Is Valid`
            (set `self.PreviousLength` (`KismetMathLibrary.VSize` (`self.GetVelocity` (`self.Player`))))
            (set `/Game/Unreal_Asset/ThirdPerson/Blueprints/BP_ThirdPersonCharacter.CanTeleport?` false (`self.Player`))
            (`self.K2_SetActorTransform` (`GameplayStatics.GetPlayerCharacter` 0) (`KismetMathLibrary.MakeTransform` (`SceneComponent.K2_GetComponentLocation` (`Actor.RootComponent` _exitportalpassive)) (`SceneComponent.K2_GetComponentRotation` (`Actor.RootComponent` _exitportalpassive))) false true)
            (`Character.LaunchCharacter` (`self.Player`) (* (`SceneComponent.GetForwardVector` (`Actor.RootComponent` (`self.ExitPortalPassive`))) (`self.PreviousLength`)) true true)
            (`KismetSystemLibrary.Delay` 0.2)
            (set `/Game/Unreal_Asset/ThirdPerson/Blueprints/BP_ThirdPersonCharacter.CanTeleport?` true (`self.Player`))))))))

(fn `UserConstructionScript`)