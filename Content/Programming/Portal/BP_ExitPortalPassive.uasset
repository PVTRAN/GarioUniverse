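; Exit half of a passive portal pair that teleports the player to its linked entry portal on overlap.
; If an attach target is set, BeginPlay attaches to it, creates a render target for its own PortalView and shows the entry portal's view on its cylinder via dynamic material.
; Teleporting launches the player along the entry's forward vector using prior speed, with a brief CanTeleport lockout preventing immediate re-entry.
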(event `self.ReceiveTick`
  (params (DeltaSeconds :type "Float (single-precision)")))

(event `self.ReceiveBeginPlay`
  (bind _attched_to_this_actor (`self.Attched to this actor`))
  (bind _cylinder (`self.Cylinder`))
  (bind _asbp_third_person_character (cast `/Game/Unreal_Asset/ThirdPerson/Blueprints/BP_ThirdPersonCharacter` (`GameplayStatics.GetPlayerCharacter` 0)))
  (set `self.Player` _asbp_third_person_character)
  (`/Engine/EditorBlueprintResources/StandardMacros.IsValid` _attched_to_this_actor
    (:`Is Valid`
      (`self.K2_AttachToActor` _attched_to_this_actor "None" "KeepWorld" "KeepRelative" "KeepWorld")
      (bind _returnvalue (`PrimitiveComponent.CreateDynamicMaterialInstance` _cylinder 0 "/Game/Programming/Portal/Portal_Mat.Portal_Mat" "Texture"))
      (`PrimitiveComponent.SetMaterial` _cylinder 0 _returnvalue)
      (bind _returnvalue_2 (`CanvasRenderTarget2D.CreateCanvasRenderTarget2D` "/Script/Engine.CanvasRenderTarget2D"))
      (set `SceneCaptureComponent2D.TextureTarget` _returnvalue_2 (`self.PortalView`))
      (bind _returnvalue_3 (`PrimitiveComponent.CreateDynamicMaterialInstance` (`self.Cylinder`) 0 "/Game/Programming/Portal/Portal_Mat.Portal_Mat" "None"))
      (`MaterialInstanceDynamic.SetTextureParameterValue` _returnvalue_3 "Texture" (`SceneCaptureComponent2D.TextureTarget` (`/Game/Programming/Portal/BP_PortalPassive.PortalView` (`self.EntryPortalPassive`)))))))

(event `self.Exit.OnComponentBeginOverlap`
  (params (OverlappedComponent :type "PrimitiveComponent Object Reference") (OtherActor :type "Actor Object Reference") (OtherComp :type "PrimitiveComponent Object Reference") (OtherBodyIndex :type Integer) (bFromSweep :type Boolean) (SweepResult :type "HitResult Structure (by ref)"))
  (bind _entryportalpassive (`self.EntryPortalPassive`))
  (if (`/Game/Unreal_Asset/ThirdPerson/Blueprints/BP_ThirdPersonCharacter.CanTeleport?` (`self.Player`))
    (if (== OtherActor (`GameplayStatics.GetPlayerCharacter` 0))
      (`/Engine/EditorBlueprintResources/StandardMacros.IsValid` _entryportalpassive
        (:`Is Valid`
          (set `self.PreviousLength` (`KismetMathLibrary.VSize` (`self.GetVelocity` (`self.Player`))))
          (set `/Game/Unreal_Asset/ThirdPerson/Blueprints/BP_ThirdPersonCharacter.CanTeleport?` false (`self.Player`))
          (`self.K2_SetActorTransform` (`GameplayStatics.GetPlayerCharacter` 0) (`KismetMathLibrary.MakeTransform` (`SceneComponent.K2_GetComponentLocation` (`Actor.RootComponent` _entryportalpassive)) (`SceneComponent.K2_GetComponentRotation` (`Actor.RootComponent` _entryportalpassive))) false true)
          (`Character.LaunchCharacter` (`self.Player`) (* (`SceneComponent.GetForwardVector` (`Actor.RootComponent` (`self.EntryPortalPassive`))) (`self.PreviousLength`)) false false)
          (`KismetSystemLibrary.Delay` 0.2)
          (set `/Game/Unreal_Asset/ThirdPerson/Blueprints/BP_ThirdPersonCharacter.CanTeleport?` true (`self.Player`))
          (bind _returnvalue (`PrimitiveComponent.CreateDynamicMaterialInstance` (`self.Cylinder`) 0 "/Game/Programming/Portal/Portal_Mat.Portal_Mat" "None"))
          (`MaterialInstanceDynamic.SetTextureParameterValue` _returnvalue "Texture" (`SceneCaptureComponent2D.TextureTarget` (`/Game/Programming/Portal/BP_PortalPassive.PortalView` (`self.EntryPortalPassive`)))))))))

(fn `UserConstructionScript`)