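; Exit portal actor that teleports the player to an entry portal when they overlap its Exit component.
; It targets the player's current EntryPortal, or its own EntryPortalPassive when flagged IsPassive.
; The player is moved to that portal's location and rotation and launched along its forward vector.
; The player's CanTeleport flag is cleared for a short delay to prevent immediate re-triggering.
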(event `self.ReceiveTick`
  (params (DeltaSeconds :type "Float (single-precision)")))

(event `self.ReceiveBeginPlay`
  (bind _asbp_third_person_character (cast `/Game/Unreal_Asset/ThirdPerson/Blueprints/BP_ThirdPersonCharacter` (`GameplayStatics.GetPlayerCharacter` 0)))
  (set `self.Player` _asbp_third_person_character))

(event `self.Exit.OnComponentBeginOverlap`
  (params (OverlappedComponent :type "PrimitiveComponent Object Reference") (OtherActor :type "Actor Object Reference") (OtherComp :type "PrimitiveComponent Object Reference") (OtherBodyIndex :type Integer) (bFromSweep :type Boolean) (SweepResult :type "HitResult Structure (by ref)"))
  (bind _entryportalpassive (`self.EntryPortalPassive`))
  (bind _entryportal (`/Game/Unreal_Asset/ThirdPerson/Blueprints/BP_ThirdPersonCharacter.EntryPortal` (`self.Player`)))
  (if (`/Game/Unreal_Asset/ThirdPerson/Blueprints/BP_ThirdPersonCharacter.CanTeleport?` (`self.Player`))
    (if (== OtherActor (`GameplayStatics.GetPlayerCharacter` 0))
      (if (not (`self.IsPassive?`))
        (`/Engine/EditorBlueprintResources/StandardMacros.IsValid` _entryportal
          (:`Is Valid`
            (set `/Game/Unreal_Asset/ThirdPerson/Blueprints/BP_ThirdPersonCharacter.CanTeleport?` false (`self.Player`))
            (`self.K2_SetActorTransform` (`GameplayStatics.GetPlayerCharacter` 0) (`KismetMathLibrary.MakeTransform` (`SceneComponent.K2_GetComponentLocation` (`Actor.RootComponent` _entryportal)) (`SceneComponent.K2_GetComponentRotation` (`Actor.RootComponent` _entryportal))) false true)
            (`Character.LaunchCharacter` (`self.Player`) (* (`SceneComponent.GetForwardVector` (`Actor.RootComponent` (`/Game/Unreal_Asset/ThirdPerson/Blueprints/BP_ThirdPersonCharacter.EntryPortal` (`self.Player`)))) 1000.0) false false)
            (`KismetSystemLibrary.Delay` 0.2)
            (set `/Game/Unreal_Asset/ThirdPerson/Blueprints/BP_ThirdPersonCharacter.CanTeleport?` true (`self.Player`))))
        (else
          (`/Engine/EditorBlueprintResources/StandardMacros.IsValid` _entryportalpassive
            (:`Is Valid`
              (set `/Game/Unreal_Asset/ThirdPerson/Blueprints/BP_ThirdPersonCharacter.CanTeleport?` false (`self.Player`))
              (`self.K2_SetActorTransform` (`GameplayStatics.GetPlayerCharacter` 0) (`KismetMathLibrary.MakeTransform` (`SceneComponent.K2_GetComponentLocation` (`Actor.RootComponent` _entryportalpassive)) (`SceneComponent.K2_GetComponentRotation` (`Actor.RootComponent` _entryportalpassive))) false true)
              (`Character.LaunchCharacter` (`self.Player`) (* (`SceneComponent.GetForwardVector` (`Actor.RootComponent` (`self.EntryPortalPassive`))) 1000.0) false false)
              (`KismetSystemLibrary.Delay` 0.2)
              (set `/Game/Unreal_Asset/ThirdPerson/Blueprints/BP_ThirdPersonCharacter.CanTeleport?` true (`self.Player`)))))))))

(fn `UserConstructionScript`)