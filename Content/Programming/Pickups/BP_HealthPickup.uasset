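; Health pickup actor that heals the player and destroys itself when its pickup component is overlapped.
; The overlap triggers a heal event, plays a pickup sound at the actor's location, then destroys the actor.
; Healing works by applying negative damage to player character 0, whatever actor overlapped, after sending that character a heal message; the amount is also printed on screen.
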(event `self.ThisOnPickupComponent.OnComponentBeginOverlap`
  (params (OverlappedComponent :type "PrimitiveComponent Object Reference") (OtherActor :type "Actor Object Reference") (OtherComp :type "PrimitiveComponent Object Reference") (OtherBodyIndex :type Integer) (bFromSweep :type Boolean) (SweepResult :type "HitResult Structure (by ref)"))
  (`/Game/Programming/HealthSystem/BPI_HealthManagement.HealAmount` (`self.NegativeDamage(Healing)`))
  (`GameplayStatics.PlaySoundAtLocation` "/Game/Audio/SFX/HealthPickup.HealthPickup" (`self.K2_GetActorLocation`) (struct) 1.0 1.0 0.0 null null null null)
  (`self.K2_DestroyActor`))

(event `self.HealAmount`
  (params (healthAdjustable :type "Float (double-precision)"))
  (`self.PrintHealthPickedUp`))

(fn `PrintHealthPickedUp`
  ;[0 0 0] Function is called on the player
  (message `/Game/Programming/HealthSystem/BPI_HealthManagement.HealAmount` (`GameplayStatics.GetPlayerCharacter` 0) (`self.NegativeDamage(Healing)`))
  (`GameplayStatics.ApplyDamage` (`GameplayStatics.GetPlayerCharacter` 0) (`self.NegativeDamage(Healing)`))
  (`KismetSystemLibrary.PrintString` (`KismetStringLibrary.Conv_DoubleToString` (`self.NegativeDamage(Healing)`))))

(fn `UserConstructionScript`)