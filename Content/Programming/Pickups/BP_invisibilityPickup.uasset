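; One-shot invisibility pickup that temporarily toggles invisibility on an overlapping player character.
; Overlap with a BPI_PlayerCharacter implementer sends the toggle message, disables collision, hides the pickup and plays the HealthPickup sound.
; A MaxTimer-length timer then sends the opposite toggle to end invisibility.
; An unreferenced PrintHealthPickedUp function holds separate healing logic using negative damage on player zero.
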(event `self.ThisOnPickupComponent.OnComponentBeginOverlap`
  (params (OverlappedComponent :type "PrimitiveComponent Object Reference") (OtherActor :type "Actor Object Reference") (OtherComp :type "PrimitiveComponent Object Reference") (OtherBodyIndex :type Integer) (bFromSweep :type Boolean) (SweepResult :type "HitResult Structure (by ref)"))
  (if (`KismetSystemLibrary.DoesImplementInterface` OtherActor "/Game/Unreal_Asset/ThirdPerson/Blueprints/BPI_PlayerCharacter.BPI_PlayerCharacter_C")
    (`/Engine/EditorBlueprintResources/StandardMacros.DoOnce` false
      (:`Completed`
        (message `/Game/Unreal_Asset/ThirdPerson/Blueprints/BPI_PlayerCharacter.Toggle invisibility` OtherActor false)
        (`PrimitiveComponent.SetCollisionEnabled` (`self.ThisOnPickupComponent`) "NoCollision")
        (`SceneComponent.SetHiddenInGame` (`self.invisibility_pickup`) true false)
        (`GameplayStatics.PlaySoundAtLocation` "/Game/Audio/SFX/HealthPickup.HealthPickup" (`self.K2_GetActorLocation`) (struct) 1.0 1.0 0.0 null null null null)
        (`KismetSystemLibrary.K2_SetTimerDelegate` (delegate `disable invisability`) (`self.Max_Timer`))))))

(event `disable invisability`
  (message `/Game/Unreal_Asset/ThirdPerson/Blueprints/BPI_PlayerCharacter.Toggle invisibility` (stale `self.ThisOnPickupComponent.OnComponentBeginOverlap` OtherActor) true))

(fn `PrintHealthPickedUp`
  ;[0 0 0] Function is called on the player
  (message `/Game/Programming/HealthSystem/BPI_HealthManagement.HealAmount` (`GameplayStatics.GetPlayerCharacter` 0) (`self.NegativeDamage(Healing)`))
  (`GameplayStatics.ApplyDamage` (`GameplayStatics.GetPlayerCharacter` 0) (`self.NegativeDamage(Healing)`))
  (`KismetSystemLibrary.PrintString` (`KismetStringLibrary.Conv_DoubleToString` (`self.NegativeDamage(Healing)`))))

(fn `UserConstructionScript`)