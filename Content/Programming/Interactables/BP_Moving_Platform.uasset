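; Interactable moving platform that travels between a begin and an end location when its IsActive flag is set.
; BeginPlay and an overlap by player character 0 both check the flag, then play the Move timeline.
; The timeline's track drives a lerp between the two location variables, setting the root's world location without sweep.
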(event `self.ReceiveBeginPlay`
  ;[1 1 1] Move Platform if Active
  (if (`self.IsActive?`) :!label _label
    (bind (_direction _newtrack_0) (`Timeline|Move`)
      (:`Update`
        (`SceneComponent.K2_SetWorldLocation` (`self.DefaultSceneRoot`) (`KismetMathLibrary.VLerp` (`self.ActorBeginLocation`) (`self.ActorEndLocation`) _newtrack_0) false false)))))

(event `self.ReceiveActorBeginOverlap`
  (params (OtherActor :type "Actor Object Reference"))
  ;[1 1 1] Move Platform if Active
  (if (== OtherActor (`GameplayStatics.GetPlayerCharacter` 0))
    (goto _label)))

(fn `UserConstructionScript`)