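; Interactable door that swings open and closed on alternate Interact calls, printing "Locked" instead when it is locked.
; A FlipFlop plays or reverses the DoorOpen timeline, which lerps the Cube's world rotation between stored begin and end rotations.
; A recently-triggered flag blocks repeat use until a short Delay, started from the timeline update, clears it.
; The Box overlap shows and removes an interact prompt widget for the player.
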(event `/Game/Programming/Character/I_Interact.Interact`
  ;[1 1 1] DoorMovement
  (if (`self.HasBeenRecentlyTriggered?`)
    _
    (elif (`self.IsLocked?`)
      (`KismetSystemLibrary.PrintString` "Locked")
      (else
        (set `self.HasBeenRecentlyTriggered?` true)
        (`/Engine/EditorBlueprintResources/StandardMacros.FlipFlop`
          (:`A`
            (bind (_direction _newtrack_0) (`Timeline|Door Open` :!label _label)
              (:`Update`
                (`SceneComponent.K2_SetWorldRotation` (`self.Cube`) (`KismetMathLibrary.RLerp` (`self.ActorBeginRotation`) (`self.ActorEndRotation`) _newtrack_0) false false)
                (`KismetSystemLibrary.Delay` 1.0)
                (set `self.HasBeenRecentlyTriggered?` false))))
          (:`B`
            (goto _label :!via `ReverseFromEnd`)))))))

(event `self.Box.OnComponentBeginOverlap`
  (params (OverlappedComponent :type "PrimitiveComponent Object Reference") (OtherActor :type "Actor Object Reference") (OtherComp :type "PrimitiveComponent Object Reference") (OtherBodyIndex :type Integer) (bFromSweep :type Boolean) (SweepResult :type "HitResult Structure (by ref)"))
  (if (== OtherActor (`GameplayStatics.GetPlayerCharacter` 0))
    (bind _returnvalue (`|CreateWidget` "/Game/Art_Asset/User_Interface/W_Interact_Prompt.W_Interact_Prompt_C" (`GameplayStatics.GetPlayerController` 0)))
    (`UserWidget.AddToViewport` _returnvalue 0)))

(event `self.Box.OnComponentEndOverlap`
  (params (OverlappedComponent :type "PrimitiveComponent Object Reference") (OtherActor :type "Actor Object Reference") (OtherComp :type "PrimitiveComponent Object Reference") (OtherBodyIndex :type Integer))
  (if (== OtherActor (`GameplayStatics.GetPlayerCharacter` 0))
    (bind _foundwidgets (`WidgetBlueprintLibrary.GetAllWidgetsOfClass` "/Game/Art_Asset/User_Interface/W_Interact_Prompt.W_Interact_Prompt_C"))
    (`Widget.RemoveFromParent` _foundwidgets)))

(fn `UserConstructionScript`)