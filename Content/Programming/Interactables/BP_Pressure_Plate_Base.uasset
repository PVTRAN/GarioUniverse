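; Pressure plate that switches linked objects on or off when weighted by a grabbable cube or the player.
; Tick line-traces upward against every BP_Grabbable_Cube, applying on or off per cube, while Box overlaps handle the player.
; Both set GravityVolume's state and toggle the first valid of Door lock, Platform or LaunchPad.
; A Timeline lerps the plate down or back between begin and end locations.
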(event `self.ReceiveTick`
  (params (DeltaSeconds :type "Float (single-precision)"))
  (bind _cube (`self.Cube`))
  (bind _door (`self.Door`))
  (bind _platform (`self.Platform`))
  (bind _launchpad (`self.LaunchPad`))
  (bind _platform_2 (`self.Platform`))
  (bind _launchpad_2 (`self.LaunchPad`))
  (bind _gravityvolume (`self.GravityVolume`))
  (bind _door_2 (`self.Door`))
  (bind _returnvalue (`SceneComponent.K2_GetComponentLocation` _cube))
  (bind _outactors (`GameplayStatics.GetAllActorsOfClass` "/Game/Programming/Interactables/BP_Grabbable_Cube.BP_Grabbable_Cube_C"))
  (for _array_element _outactors
    (bind (_hitlocation _hitnormal _bonename _outhit _returnvalue_2) (`PrimitiveComponent.K2_LineTraceComponent` (`/Game/Programming/Interactables/BP_Grabbable_Cube.Cube` _array_element) _returnvalue (+ (* (`KismetMathLibrary.GetUpVector` (`SceneComponent.K2_GetComponentRotation` _cube)) 200.0) _returnvalue) true true false))
    (if _returnvalue_2
      ;[1 1 1] Triggers or Untriggers any object it is Tied to
      (message `/Game/Programming/Gravity/BPI_Gravity_Object.SetVolumeGravityState` _gravityvolume (`self.GravityStateActivated`) :!label _label)
      (`/Engine/EditorBlueprintResources/StandardMacros.IsValid` _door
        (:`Is Valid`
          (set `/Game/Programming/Interactables/BP_Interactable_Door.IsLocked?` false _door)
          (bind (_direction _newtrack_0) (`Timeline|Timeline` :!label _label_2)
            (:`Update`
              (`SceneComponent.K2_SetWorldLocation` (`self.Cube`) (`KismetMathLibrary.VLerp` (`self.ActorBeginLocation`) (`self.ActorEndLocation`) _newtrack_0) false false))))
        (:`Is Not Valid`
          (`/Engine/EditorBlueprintResources/StandardMacros.IsValid` _platform_2
            (:`Is Valid`
              (set `/Game/Programming/Interactables/BP_Moving_Platform.IsActive?` true _platform_2)
              (goto _label_2))
            (:`Is Not Valid`
              (`/Engine/EditorBlueprintResources/StandardMacros.IsValid` _launchpad
                (:`Is Valid`
                  (set `/Game/Programming/Interactables/BP_Interactable_Launch_Pad.IsActive?` true _launchpad)
                  (goto _label_2))
                (:`Is Not Valid`
                  (goto _label_2)))))))
      (else
        (message `/Game/Programming/Gravity/BPI_Gravity_Object.SetVolumeGravityState` _gravityvolume (`self.GravityStateUnactivated`) :!label _label_3)
        (`/Engine/EditorBlueprintResources/StandardMacros.IsValid` _door_2
          (:`Is Valid`
            (set `/Game/Programming/Interactables/BP_Interactable_Door.IsLocked?` true _door_2)
            (goto _label_2 :!via `Reverse`))
          (:`Is Not Valid`
            (`/Engine/EditorBlueprintResources/StandardMacros.IsValid` _platform
              (:`Is Valid`
                (set `/Game/Programming/Interactables/BP_Moving_Platform.IsActive?` false _platform)
                (goto _label_2 :!via `Reverse`))
              (:`Is Not Valid`
                (`/Engine/EditorBlueprintResources/StandardMacros.IsValid` _launchpad_2
                  (:`Is Valid`
                    (set `/Game/Programming/Interactables/BP_Interactable_Launch_Pad.IsActive?` false _launchpad_2)
                    (goto _label_2 :!via `Reverse`))
                  (:`Is Not Valid`
                    (goto _label_2 :!via `Reverse`)))))))))))

(event `self.Box.OnComponentBeginOverlap`
  (params (OverlappedComponent :type "PrimitiveComponent Object Reference") (OtherActor :type "Actor Object Reference") (OtherComp :type "PrimitiveComponent Object Reference") (OtherBodyIndex :type Integer) (bFromSweep :type Boolean) (SweepResult :type "HitResult Structure (by ref)"))
  ;[1 1 1] Triggers or Untriggers any object it is Tied to
  (if (== OtherActor (`GameplayStatics.GetPlayerCharacter` 0))
    (goto _label)))

(event `self.Box.OnComponentEndOverlap`
  (params (OverlappedComponent :type "PrimitiveComponent Object Reference") (OtherActor :type "Actor Object Reference") (OtherComp :type "PrimitiveComponent Object Reference") (OtherBodyIndex :type Integer))
  ;[1 1 1] Triggers or Untriggers any object it is Tied to
  (if (== OtherActor (`GameplayStatics.GetPlayerCharacter` 0))
    (goto _label_3)))

(fn `UserConstructionScript`)