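; Interactable launch pad that launches the player character on overlap while its IsActive flag is set.
; The launch vector derives from the player's current velocity: X is amplified and Y is zeroed.
; Z scales the current vertical speed, using a doubled-plus-offset formula when not rising, which keeps most falling velocities pointed downward rather than bouncing them up.
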(event `self.ReceiveActorBeginOverlap`
  (params (OtherActor :type "Actor Object Reference"))
  (bind _returnvalue (`GameplayStatics.GetPlayerCharacter` 0))
  (bind (_returnvalue_x _returnvalue_y _returnvalue_z) (`KismetMathLibrary.BreakVector` (`self.GetVelocity` _returnvalue)))
  ;[1 1 1] Launch Character
  (if (== OtherActor _returnvalue)
    (if (`self.IsActive?`)
      (if (<= _returnvalue_z 0.0)
        (set `self.Launch Velocity Z` (* (+ _returnvalue_z _returnvalue_z 1.0) 20.0))
        (else
          (set `self.Launch Velocity Z` (* _returnvalue_z 20.0))))
      (`Character.LaunchCharacter` _returnvalue (`KismetMathLibrary.MakeVector` (* _returnvalue_x 10.0) (* _returnvalue_y 0.0) (`self.Launch Velocity Z`)) false false))))

(fn `UserConstructionScript`)