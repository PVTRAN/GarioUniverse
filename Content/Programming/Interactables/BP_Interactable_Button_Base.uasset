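; Base interactable button that moves when used and activates linked level objects.
; Interact plays a timeline lerping the root between begin and end locations, with a recently-triggered flag blocking repeats.
; From the timeline's Update, after a delay, it clears the flag, unlocks the door, activates the moving platform and launch pad, and toggles the fire hazard.
; Box overlap by the player shows or hides a spotlight and interact prompt.
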(event `/Game/Programming/Character/I_Interact.Interact`
  (bind _doorreference (`self.DoorReference`))
  (bind _movingplatform (`self.MovingPlatform`))
  (bind _launchpad (`self.LaunchPad`))
  ;[1 1 1] Button Movement
  (if (not (`self.HasBeenRecentlyTriggered?`))
    (set `self.HasBeenRecentlyTriggered?` true)
    (bind (_direction _newtrack_0) (`Timeline|Timeline` :!via `PlayFromStart`)
      (:`Update`
        (`SceneComponent.K2_SetWorldLocation` (`self.DefaultSceneRoot`) (`KismetMathLibrary.VLerp` (`self.ActorBeginLocation`) (`self.ActorEndLocation`) _newtrack_0) false false)
        (`KismetSystemLibrary.Delay` 2.0)
        (set `self.HasBeenRecentlyTriggered?` false)
        (`/Engine/EditorBlueprintResources/StandardMacros.IsValid` _doorreference
          (:`Is Valid`
            (set `/Game/Programming/Interactables/BP_Interactable_Door.IsLocked?` false _doorreference))
          (:`Is Not Valid`
            _))
        (`/Engine/EditorBlueprintResources/StandardMacros.IsValid` _movingplatform
          (:`Is Valid`
            (set `/Game/Programming/Interactables/BP_Moving_Platform.IsActive?` true _movingplatform))
          (:`Is Not Valid`
            _))
        (`/Engine/EditorBlueprintResources/StandardMacros.IsValid` _launchpad
          (:`Is Valid`
            (set `/Game/Programming/Interactables/BP_Interactable_Launch_Pad.IsActive?` true _launchpad))
          (:`Is Not Valid`
            _))
        (message `/Game/Programming/Gameplay/Obstacles_and_Traps/BI_Toggle_On_Off.Toggle` (`self.FireHazard`))))))

(event `self.Box.OnComponentBeginOverlap`
  (params (OverlappedComponent :type "PrimitiveComponent Object Reference") (OtherActor :type "Actor Object Reference") (OtherComp :type "PrimitiveComponent Object Reference") (OtherBodyIndex :type Integer) (bFromSweep :type Boolean) (SweepResult :type "HitResult Structure (by ref)"))
  ;[1 1 1] Light Up Button When Close Enough to Interact
  (if (== OtherActor (`GameplayStatics.GetPlayerCharacter` 0))
    (if (not (`self.HasBeenRecentlyTriggered?`))
      (`SceneComponent.SetHiddenInGame` (`self.SpotLight`) false false)
      (bind _returnvalue (`|CreateWidget` "/Game/Art_Asset/User_Interface/W_Interact_Prompt.W_Interact_Prompt_C" (`GameplayStatics.GetPlayerController` 0)))
      (`UserWidget.AddToViewport` _returnvalue 0))))

(event `self.Box.OnComponentEndOverlap`
  (params (OverlappedComponent :type "PrimitiveComponent Object Reference") (OtherActor :type "Actor Object Reference") (OtherComp :type "PrimitiveComponent Object Reference") (OtherBodyIndex :type Integer))
  ;[1 1 1] Turn Light Off When Not Close Enough to Interact
  (if (== OtherActor (`GameplayStatics.GetPlayerCharacter` 0))
    (`SceneComponent.SetHiddenInGame` (`self.SpotLight`) true false)
    (bind _foundwidgets (`WidgetBlueprintLibrary.GetAllWidgetsOfClass` "/Game/Art_Asset/User_Interface/W_Interact_Prompt.W_Interact_Prompt_C"))
    (`Widget.RemoveFromParent` _foundwidgets)))

(fn `UserConstructionScript`)