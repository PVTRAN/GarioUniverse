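; BP_BlackHole is a black hole hazard that applies radial force and kills or destroys what enters its death field.
; On BeginPlay it sets the force radius, then a looping timer repeatedly fires a radial impulse as gravity.
; Death field overlaps trigger brief slow motion and the game mode's death message for the player; other actors are destroyed after a delay.
; An unconnected branch would spawn a BP_Gravity_Base volume but never runs.
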(event `self.ReceiveBeginPlay`
  (set `RadialForceComponent.Radius` (`self.Radius`) (`self.RadialForce`))
  (`KismetSystemLibrary.K2_SetTimer` null "Gravity" 0.1 true))

(event `self.DeathField.OnComponentBeginOverlap`
  (params (OverlappedComponent :type "PrimitiveComponent Object Reference") (OtherActor :type "Actor Object Reference") (OtherComp :type "PrimitiveComponent Object Reference") (OtherBodyIndex :type Integer) (bFromSweep :type Boolean) (SweepResult :type "HitResult Structure (by ref)"))
  (if (== OtherActor (`GameplayStatics.GetPlayerCharacter` 0))
    (`GameplayStatics.SetGlobalTimeDilation` 0.3)
    (`KismetSystemLibrary.Delay` 0.25)
    (`GameplayStatics.SetGlobalTimeDilation` 1.0)
    (message `/Game/BPI_Gamemode.Player Death` (`GameplayStatics.GetGameMode`))
    (else
      (`KismetSystemLibrary.Delay` 1.0)
      (`self.K2_DestroyActor` OtherActor))))

(fn `Gravity`
  (`RadialForceComponent.FireImpulse` (`self.RadialForce`)))

(fn `UserConstructionScript`)