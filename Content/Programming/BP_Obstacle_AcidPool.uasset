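; Acid pool obstacle that applies repeating damage to the player on entering its box collision.
; Overlap sets a damage flag unless all acid objects are flagged invalid, then constructs a damage UObject for the player if none is valid.
; That object receives the damage amount, interval and prolong duration through CallDamageFromClass.
; Tick draws a debug box around the collision bounds every frame.
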(event `self.ReceiveBeginPlay`)

(event `self.ReceiveTick`
  (params (DeltaSeconds :type "Float (single-precision)"))
  (bind _boxcollision (`self.BoxCollision`))
  (bind (_origin _boxextent) (`KismetSystemLibrary.GetComponentBounds` _boxcollision))
  ;[1 0.4967 0] Debug Box
  (`KismetSystemLibrary.DrawDebugBox` _origin _boxextent (struct :`G` 1.0 :`B` 0.170606 :`A` 1.0) (`SceneComponent.K2_GetComponentRotation` _boxcollision) 0.03 3.0))

(event `self.BoxCollision.OnComponentBeginOverlap`
  (params (OverlappedComponent :type "PrimitiveComponent Object Reference") (OtherActor :type "Actor Object Reference") (OtherComp :type "PrimitiveComponent Object Reference") (OtherBodyIndex :type Integer) (bFromSweep :type Boolean) (SweepResult :type "HitResult Structure (by ref)"))
  (bind _returnvalue (`GameplayStatics.GetPlayerCharacter` 0))
  ;[1 0.1458 0] OnBeginOverlapTrigger
  (`|ExecutionSequence`
    (:`then_0`
      (if (not (`self.AllAcidObjectsInvalid?`))
        (set `self.IsApplyingDamage` true)
        (if (and (== OtherActor _returnvalue) (`KismetSystemLibrary.IsValid` _returnvalue) (not (`KismetSystemLibrary.IsValid` (`self.DamageUObject`))))
          (bind _returnvalue_2 (`|GenericCreateObject` self (`self.DamageClass`)))
          (bind _output_get (set `self.DamageUObject` _returnvalue_2))
          (`/Game/Programming/BP_DamageClass.CallDamageFromClass` _output_get (`GameplayStatics.GetPlayerCharacter` 0) self (`self.DamageAmount`) (`self.DamageInterval`) (`self.DamageDuration`)))))))

(fn `UserConstructionScript`
  (`parent.UserConstructionScript`))