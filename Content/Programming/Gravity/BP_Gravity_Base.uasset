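; Gravity volume actor that pulls or pushes overlapping physics bodies using directional, radial or line-relative gravity, with off and inverted states.
; Construction adds the chosen box, sphere or capsule collider, trims debug arrows and applies the initial state.
; Tick applies mass-independent AddForce to each simulating component, disabling itself when the volume is off or empty until re-enabled.
; Overlap events also set the player character's gravity scale, zeroing it on exit.
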(event `self.ReceiveBeginPlay`
  ;[1 0 0.1157] BeginPlay
  (`|ExecutionSequence`
    (:`then_0`
      (if (`self.DebugMode?`)
        (`KismetSystemLibrary.PrintString` (`KismetStringLibrary.Concat_StrStr` "[Volume // " (`KismetSystemLibrary.GetDisplayName` self) "]: AWAKE!") true true (struct :`R` 1.0 :`B` 0.197169 :`A` 1.0) 3.0)))))

(event `self.ReceiveTick`
  (params (DeltaSeconds :type "Float (single-precision)"))
  ;[1 0 0.1157] Tick
  (`|ExecutionSequence`
    (:`then_0`
      (`self.TickDelegate_GravityUpdate`)
      (`KismetSystemLibrary.PrintString` (`KismetStringLibrary.Concat_StrStr` "[" (`KismetSystemLibrary.GetDisplayName` self) "]: " " \n[GravityToggles]: " (`KismetStringLibrary.Conv_BoolToString` (`self.GravityToggledOff?`))) true true (struct :`G` 1.0 :`B` 0.402706 :`A` 1.0) 0.001))))

(event `TickDelegate_GravityUpdate`
  ;[0.03675 0 1] Gravity Function
  ;;[0 0 0 1 20] DO NOT TOUCH
  (`self.GravityCalculator`))

(event `self.ReceiveActorBeginOverlap`
  (params (OtherActor :type "Actor Object Reference"))
  (bind _returnvalue (`GameplayStatics.GetPlayerCharacter` 0))
  ;[1 0 0.148] OverlapEvents
  (`|ExecutionSequence`
    (:`then_0`
      (`self.AttemptEnableGravity`)
      (if (== OtherActor _returnvalue)
        (message `/Game/Unreal_Asset/ThirdPerson/Blueprints/BPI_PlayerCharacter.SetGravityScale` _returnvalue (* (`self.Gravity Scale Player`) (`KismetMathLibrary.SelectFloat` -1.0 1.0 (`self.InvertGravity?`))))))))

(event `self.ReceiveActorEndOverlap`
  (params (OtherActor :type "Actor Object Reference"))
  (bind _returnvalue (`GameplayStatics.GetPlayerCharacter` 0))
  ;[1 0 0.148] OverlapEvents
  (`|ExecutionSequence`
    (:`then_0`
      (if (== OtherActor _returnvalue)
        (message `/Game/Unreal_Asset/ThirdPerson/Blueprints/BPI_PlayerCharacter.SetGravityScale` _returnvalue 0.0)))))

(event `/Game/Programming/Gravity/BPI_Gravity_Object.SetVolumeGravityState`
  (params (`ToggleOn?` :type "/Game/Programming/Gravity/EN_GravityState Enum" :default "NewEnumerator0"))
  ;[1 0 0.75] GravityToggle
  (switch `/Game/Programming/Gravity/EN_GravityState` `ToggleOn?`
    (:`NewEnumerator0`
      (set `self.GravityToggledOff?` true))
    (:`NewEnumerator1`
      (set `self.GravityToggledOff?` false)
      (`self.AttemptEnableGravity`))
    (:`NewEnumerator2`
      (set `self.InvertGravity?` true))
    (:`NewEnumerator3`
      (set `self.InvertGravity?` false))))

(fn `AddCollisionByType`
  (params (Collision :type "/Game/Programming/Gravity/EN_GravityCollisionShapes Enum" :default "NewEnumerator0"))
  (locals (`SuccessfullyAttached?` :type Boolean))
  (bind (_returnvalue_location _returnvalue_rotation) (`KismetMathLibrary.BreakTransform` (`SceneComponent.GetRelativeTransform` (`self.GravityRoot`))))
  (`|ExecutionSequence`
    (:`then_0`
      ;[1 0.2186 0] Collision Types
      (switch `/Game/Programming/Gravity/EN_GravityCollisionShapes` Collision
        (:`NewEnumerator0`
          (bind _returnvalue (`AddComponent|NODE_AddBoxComponent-1` :`bManualAttachment` true :`RelativeTransform` (`KismetMathLibrary.MakeTransform` _returnvalue_location _returnvalue_rotation (`self.GravityVolumeScale`))))
          (bind _output_get (set `self.BPC_BoxCollider` _returnvalue))
          (set `PrimitiveComponent.bGenerateOverlapEvents` true _output_get))
        (:`NewEnumerator1`
          (bind _returnvalue_2 (`AddComponent|NODE_AddSphereComponent-0` :`bManualAttachment` true :`RelativeTransform` (`KismetMathLibrary.MakeTransform` _returnvalue_location _returnvalue_rotation (`self.GravityVolumeScale`))))
          (bind _output_get_2 (set `self.BPC_SphereCollider` _returnvalue_2))
          (set `PrimitiveComponent.bGenerateOverlapEvents` true _output_get_2))
        (:`NewEnumerator2`
          (bind _returnvalue_3 (`AddComponent|NODE_AddCapsuleComponent-0` :`bManualAttachment` true :`RelativeTransform` (`KismetMathLibrary.MakeTransform` _returnvalue_location _returnvalue_rotation (`self.GravityVolumeScale`))))
          (bind _output_get_3 (set `self.BPC_CapsuleCollider` _returnvalue_3))
          (set `PrimitiveComponent.bGenerateOverlapEvents` true _output_get_3))))
    (:`then_1`
      (return))))

(fn `AttemptEnableGravity`
  (if (and (`KismetMathLibrary.BooleanNOR` (`self.GravityToggledOff?`) (< (`KismetArrayLibrary.Array_Length` (`self.GetOverlappingComponents`)) 1)) (not (`self.IsActorTickEnabled`)))
    (`self.SetActorTickEnabled` true)))

(fn `GetDirectionalGravityVector`
  (returns (`Directional Vector` :type "Vector Structure"))
  (bind _gravitystrength (`self.GravityStrength`))
  (return (* (`self.GetActorUpVector`) (`KismetMathLibrary.SelectFloat` (* _gravitystrength -1.0) _gravitystrength (`self.InvertGravity?`)))))

(fn `GetPointRelativeLineVector`
  (params (SceneComponent :type "SceneComponent Object Reference") (`IncludeLineEndPoints?` :type Boolean))
  (returns (PointRelativeLineVector :type "Vector Structure") (PointOnLine_Location :type "Vector Structure") (EndPoint_1 :type "Vector Structure") (EndPoint_2 :type "Vector Structure"))
  (bind _returnvalue (`SceneComponent.K2_GetComponentLocation` SceneComponent))
  (bind _includelineendpoints_ (`local.IncludeLineEndPoints?`))
  (bind _pointrelativeline_length (`self.PointRelativeLine_Length`))
  (bind _gravityroot (`self.GravityRoot`))
  (bind _gravitystrength (`self.GravityStrength`))
  (bind _returnvalue_2 (`SceneComponent.K2_GetComponentLocation` _gravityroot))
  (bind _returnvalue_3 (`SceneComponent.GetRightVector` _gravityroot))
  (bind _returnvalue_4 (`KismetMathLibrary.SelectFloat` (* _gravitystrength -1.0) _gravitystrength (`self.InvertGravity?`)))
  (bind _returnvalue_5 (`KismetMathLibrary.FindClosestPointOnLine` _returnvalue _returnvalue_2 _returnvalue_3))
  (bind _returnvalue_6 (+ (* _returnvalue_3 (* _pointrelativeline_length -1.0)) _returnvalue_2))
  (bind _returnvalue_7 (+ _returnvalue_2 (* _returnvalue_3 _pointrelativeline_length)))
  (bind _returnvalue_8 (`KismetMathLibrary.FindClosestPointOnSegment` _returnvalue _returnvalue_7 _returnvalue_6))
  (return (`KismetMathLibrary.SelectVector` (* (`KismetMathLibrary.Normal` (- _returnvalue _returnvalue_8)) _returnvalue_4) (* (`KismetMathLibrary.Normal` (- _returnvalue _returnvalue_5)) _returnvalue_4) _includelineendpoints_) (`KismetMathLibrary.SelectVector` _returnvalue_8 _returnvalue_5 _includelineendpoints_) _returnvalue_7 _returnvalue_6))

(fn `GetRadialGravityVector`
  (params (SceneComponent :type "SceneComponent Object Reference"))
  (returns (`Radial Vector` :type "Vector Structure"))
  (bind _gravitystrength (`self.GravityStrength`))
  (return (* (`KismetMathLibrary.Normal` (- (`SceneComponent.K2_GetComponentLocation` SceneComponent) (`SceneComponent.K2_GetComponentLocation` (`self.GravityRoot`)))) (`KismetMathLibrary.SelectFloat` (* _gravitystrength -1.0) _gravitystrength (`self.InvertGravity?`)))))

(fn `GravityCalculator`
  (bind _overlappingcomponents (`self.GetOverlappingComponents`))
  (bind _gravityalignment_setting (`self.GravityAlignment_Setting`))
  (bind _returnvalue (`SceneComponent.K2_GetComponentLocation` (`self.GravityRoot`)))
  ;[0.2555 0 1] Gravity Function
  (if (`KismetMathLibrary.BooleanNOR` (`self.GravityToggledOff?`) (< (`KismetArrayLibrary.Array_Length` _overlappingcomponents) 1))
    (for _array_element _overlappingcomponents
      (if (and (`SceneComponent.IsSimulatingPhysics` _array_element "None") (`KismetSystemLibrary.IsValid` _array_element))
        (bind (_pointrelativelinevector _pointonline_location _endpoint_1 _endpoint_2) (`self.GetPointRelativeLineVector` _array_element (`self.GravityLineEndPointsEnabled?`)))
        (bind _returnvalue_2 (select `/Game/Programming/Gravity/EN_GravityAlignment` (`self.GravityAlignment_Setting`) :`NewEnumerator1` (`self.GetDirectionalGravityVector`) :`NewEnumerator0` (`self.GetRadialGravityVector` _array_element) :`NewEnumerator2` _pointrelativelinevector))
        (`PrimitiveComponent.AddForce` _array_element _returnvalue_2 "None" true)
        (if (`self.DebugMode?`)
          (bind _returnvalue_3 (`SceneComponent.K2_GetComponentLocation` _array_element))
          (`KismetSystemLibrary.DrawDebugSphere` _returnvalue_3 75.0 8 (struct :`G` 0.982318 :`B` 1.0 :`A` 1.0) 0.05 3.0)
          (`KismetSystemLibrary.DrawDebugLine` _returnvalue_3 (+ _returnvalue_3 _returnvalue_2) (struct :`R` 0.430812 :`B` 1.0 :`A` 1.0) 0.05 3.0)
          (`KismetSystemLibrary.DrawDebugSphere` (select `/Game/Programming/Gravity/EN_GravityAlignment` _gravityalignment_setting :`NewEnumerator1` _returnvalue :`NewEnumerator0` _returnvalue :`NewEnumerator2` _pointonline_location) 150.0 8 (struct :`R` 1.0 :`B` 0.227317 :`A` 1.0) 0.05 3.0)
          (switch `/Game/Programming/Gravity/EN_GravityAlignment` _gravityalignment_setting
            (:`NewEnumerator1`
              (`KismetSystemLibrary.DrawDebugSphere` (+ _returnvalue (`self.GetDirectionalGravityVector`)) 150.0 8 (struct :`R` 1.0 :`B` 0.227317 :`A` 1.0) 0.05 3.0))
            (:`NewEnumerator2`
              (`KismetSystemLibrary.DrawDebugLine` _endpoint_1 _endpoint_2 (struct :`R` 1.0 :`B` 0.226966 :`A` 1.0)))))))
    (else
      (`self.SetActorTickEnabled` false))))

(fn `SetComponentsHiddenInGame`
  (bind _returnvalue (not (`self.DebugMode?`)))
  (switch `/Game/Programming/Gravity/EN_GravityCollisionShapes` (`self.CollisionShapeForVolume`)
    (:`NewEnumerator0`
      (`SceneComponent.SetHiddenInGame` (`self.BPC_BoxCollider`) _returnvalue true))
    (:`NewEnumerator1`
      (`SceneComponent.SetHiddenInGame` (`self.BPC_SphereCollider`) _returnvalue true))
    (:`NewEnumerator2`
      (`SceneComponent.SetHiddenInGame` (`self.BPC_CapsuleCollider`) _returnvalue true))))

(fn `SetDebugArrowsByGravityAlignment`
  (`|ExecutionSequence`
    (:`then_0`
      ;[0 0.7677 1] Sort Arrows By Alignment
      (switch `/Game/Programming/Gravity/EN_GravityAlignment` (`self.GravityAlignment_Setting`)
        (:`NewEnumerator1`
          (for _array_element (`|MakeArray` (`self.Directional_Arrow_X-`) (`self.Directional_Arrow_X+`) (`self.Directional_Arrow_Y-`) (`self.Directional_Arrow_Y+`))
            (`ActorComponent.K2_DestroyComponent` _array_element)))
        (:`NewEnumerator2`
          (for _array_element_2 (`|MakeArray` (`self.Directional_Arrow_Y+`) (`self.Directional_Arrow_Y-`))
            (`ActorComponent.K2_DestroyComponent` _array_element_2)))))
    (:`then_1`
      (return))))

(fn `UserConstructionScript`
  ;[0.8551 0 1] Construct
  (`|ExecutionSequence`
    (:`then_0`
      (`|ExecutionSequence`
        (:`then_0`
          (`self.AddCollisionByType` (`self.CollisionShapeForVolume`))
          (`self.SetDebugArrowsByGravityAlignment`)
          (`self.SetActorTickEnabled` (select `/Game/Programming/Gravity/EN_GravityState` (`self.GravityState`) :`NewEnumerator1` true :`NewEnumerator2` true :`NewEnumerator3` true)))
        (:`then_1`
          (`self.SetComponentsHiddenInGame`))
        (:`then_2`
          (`/Game/Programming/Gravity/BPI_Gravity_Object.SetVolumeGravityState` (`self.GravityState`)))))))