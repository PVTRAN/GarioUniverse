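; BP_Alien is an enemy character Blueprint whose only active behavior is an idle hover effect.
; Each Tick, CalculateIdleHover sets the spring arm length by feeding a game-time sine, computed in a math expression, into a sinusoidal in-out ease.
; CalculateGravityResponse is an unfinished stub that checks for overlapping BP_Gravity_Base actors, does nothing with the result and is never called.
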(event EventBeginPlay)

(event EventTick
  (params (DeltaSeconds :type Float%20%28single-precision%29))
  (Tools|CalculateIdleHover))

(fn ConstructionScript)

(fn CalculateIdleHover
  (Utilities|FlowControl|Sequence
    (:then_0
      ;[1 0.3045 0] SIn Equation
      (Variables|/Script/Engine.SpringArmComponent|SetTargetArmLength (Variables|Default|GetSpringArm) (Math|Interpolation|Ease "SinusoidalInOut" (|((sin(x))/y) (Utilities|Time|GetGameTimeinSeconds) 2.0) 5e+01 1e+02)))
    (:then_1
      (return))))

(fn CalculateGravityResponse
  (Utilities|FlowControl|Sequence
    (:then_0
      (if (Utilities|Array|IsEmpty (Collision|GetOverlappingActors "/Game/StarterContent/Blueprints/Assets/Gravity_Blueprints/Gravity_Class_Defaults/BP_Gravity_Base.BP_Gravity_Base_C" :!class /Script/Engine.Actor))
        _))
    (:then_1
      (return))))