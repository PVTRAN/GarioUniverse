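; BP_Enemy_Alien is an alien enemy character with custom gravity direction and an idle hover.
; Gravity events store the alignment and volume, interpolate the CharacterMovement gravity direction toward that vector on each call, and set gravity scale, with getters for alignment and scale.
; Tick eases spring arm length with a sine of lifetime to create the hover.
; DebugMode prints a wake message and shows the capsule at BeginPlay.
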(event EventBeginPlay
  (if (Variables|Tools|GetDebugMode?)
    (Development|PrintString (Utilities|String|Append "[" (Utilities|GetDisplayName self) "]:" " Awake!") true true "(R=1.000000,G=0.000000,B=0.765654,A=1.000000)" 5.0)
    (Development|SetHiddeninGame (Variables|Collision|GetCapsuleComponent) (not (Variables|Tools|GetDebugMode?)) false)))

(event EventTick
  (params (DeltaSeconds :type Float%20%28single-precision%29))
  ;[1 0.3468 0] Tick
  (CallFunction|CalculateIdleHover 2.0))

(event EventSetGravityAlignment
  (params (GravitVector :type Vector :default "0, 0, 0") (GravityVolume :type Actor%20Object%20Reference))
  (Variables|Gravity|SetCurrent%20Gravity%20Alignment GravitVector)
  (Variables|Gravity|SetGravity%20Volume GravityVolume)
  (Class|CharacterMovementComponent|SetGravityDirection (Variables|Character|GetCharacterMovement) (Math|Vector|Normalize (Math|Interpolation|VInterpTo (Class|CharacterMovementComponent|GetGravityDirection (Variables|Character|GetCharacterMovement)) (Variables|Gravity|GetCurrent%20Gravity%20Alignment) (Utilities|Time|GetWorldDeltaSeconds) 4.5))))

(event EventSetGravityScale
  (params (Scale%20[Normalized] :type Float%20%28double-precision%29))
  (Variables|/Script/Engine.CharacterMovementComponent|SetGravityScale (Variables|Character|GetCharacterMovement) Scale%20[Normalized]))

(fn ConstructionScript)

(fn CalculateIdleHover
  (params (Sin%20Divisor :type Float%20%28double-precision%29))
  ;[0 1 0.5519] SinFunction
  (Variables|/Script/Engine.SpringArmComponent|SetTargetArmLength (Variables|Default|GetSpringArm) (Math|Interpolation|Ease "SinusoidalInOut" (|((sin(x))/y) (Actor|GetGameTimeSinceCreation) Sin%20Divisor) 5e+01 1e+02)))

(fn GetGravityAlignment
  (return (Variables|Gravity|GetCurrent%20Gravity%20Alignment)))

(fn GetGravityScale
  (return (Variables|/Script/Engine.CharacterMovementComponent|GetGravityScale (Variables|Character|GetCharacterMovement))))