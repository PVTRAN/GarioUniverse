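; BP_Interactable_Button is an interactable button that moves when used and highlights itself when the player is near.
; Interact plays a timeline lerping the root between begin and end locations, gated by a flag that a two-second delay, started from the timeline update, clears.
; Box overlap with the player shows a spotlight and prompt widget unless recently triggered; leaving hides both.
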(event `/Game/Unreal_Asset/Programming/Character/I_Interact.Interact`
  ;[1 1 1] Button Movement
  (if (not (`self.HasBeenRecentlyTriggered?`))
    (set `self.HasBeenRecentlyTriggered?` true)
    (bind (_direction _newtrack_0) (`Timeline|Timeline` :!via `PlayFromStart`)
      (:`Update`
        (`SceneComponent.K2_SetWorldLocation` (`self.DefaultSceneRoot`) (`KismetMathLibrary.VLerp` (`self.ActorBeginLocation`) (`self.ActorEndLocation`) _newtrack_0) false false)
        (`KismetSystemLibrary.Delay` 2.0)
        (set `self.HasBeenRecentlyTriggered?` false)))))

(event `self.Box.OnComponentBeginOverlap`
  (params (OverlappedComponent :type "PrimitiveComponent Object Reference") (OtherActor :type "Actor Object Reference") (OtherComp :type "PrimitiveComponent Object Reference") (OtherBodyIndex :type Integer) (bFromSweep :type Boolean) (SweepResult :type "HitResult Structure (by ref)"))
  ;[1 1 1] Light Up Button When Close Enough to Interact
  (if (== OtherActor (`GameplayStatics.GetPlayerCharacter` 0))
    (if (not (`self.HasBeenRecentlyTriggered?`))
      (`SceneComponent.SetHiddenInGame` (`self.SpotLight`) false false)
      (bind _returnvalue (`|CreateWidget` "/Game/Art_Asset/User_Interface/W_Interact_Prompt.W_Interact_Prompt_C" (`GameplayStatics.GetPlayerController` 0)))
      (`UserWidget.AddToViewport` _returnvalue 0))))

(event `self.Box.OnComponentEndOverlap`
  (params (OverlappedComponent :type "PrimitiveComponent Object Reference") (OtherActor :type "Actor Object Reference") (OtherComp :type "PrimitiveComponent Object Reference") (OtherBodyIndex :type Integer))
  ;[1 1 1] Turn Light Off When Not Close Enough to Interact
  (if (== OtherActor (`GameplayStatics.GetPlayerCharacter` 0))
    (`SceneComponent.SetHiddenInGame` (`self.SpotLight`) true false)
    (`Widget.RemoveFromParent` (stale `self.Box.OnComponentBeginOverlap` _returnvalue))))

(fn `UserConstructionScript`)