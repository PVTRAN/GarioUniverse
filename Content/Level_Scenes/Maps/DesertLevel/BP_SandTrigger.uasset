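; BP_SandTrigger is a desert-level actor that runs a timed countdown from BeginPlay and then blows up.
; A looping one-second timer decrements Countdown and prints the remaining value until it reaches zero, then clears itself.
; BlowUp fires the OnBlownUp dispatcher so bound listeners can react, then destroys the actor after a short delay.
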(event `ExplosionCountdown`
  (bind _result (`/Engine/EditorBlueprintResources/StandardMacros.DecrementInt` (`self.Countdown`))
    (:`  `
      (if (<= _result 0)
        (`self.BlowUp`)
        (`KismetSystemLibrary.K2_ClearAndInvalidateTimerHandle` (`self.CountdownTimer`))
        (else
          (`KismetSystemLibrary.PrintString` (`KismetStringLibrary.Conv_IntToString` (`self.Countdown`))))))))

(event `self.ReceiveBeginPlay`
  (bind _returnvalue (`KismetSystemLibrary.K2_SetTimerDelegate` (delegate `ExplosionCountdown`) 1.0 true))
  (set `self.CountdownTimer` _returnvalue))

(event `BlowUp`
  (`self.OnBlownUp`)
  (`KismetSystemLibrary.Delay` 1.0)
  (`self.K2_DestroyActor`))

(fn `UserConstructionScript`)