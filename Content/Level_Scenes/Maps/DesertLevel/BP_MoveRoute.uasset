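; Patrol route actor in the DesertLevel folder that exposes the points of its MoveRoute spline as waypoints.
; GetSplinePointAsWorldPosition returns the world location of the point at PatrolIndex.
; IncrementRoute advances that index and reports whether it has passed the last point, a check also exposed as HasReachedEndOfRoute.
; Progress lives on the route actor itself, with no reset or looping here, and its event graph is unused.
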(fn `GetSplinePointAsWorldPosition`
  (returns (SplineWorldLocation :type "Vector Structure"))
  (return (`SplineComponent.GetLocationAtSplinePoint` (`self.MoveRoute`) (`self.PatrolIndex`) "World")))

(fn `HasReachedEndOfRoute?`
  (returns (HasReachedEndOfRoute :type Boolean))
  (return (>= (`self.PatrolIndex`) (`SplineComponent.GetNumberOfSplinePoints` (`self.MoveRoute`)))))

(fn `IncrementRoute`
  (returns (HasReachedEndOfRoute :type Boolean))
  (bind _output_get (set `self.PatrolIndex` (+ (`self.PatrolIndex`) 1)))
  (return (>= _output_get (`SplineComponent.GetNumberOfSplinePoints` (`self.MoveRoute`)))))

(fn `UserConstructionScript`)