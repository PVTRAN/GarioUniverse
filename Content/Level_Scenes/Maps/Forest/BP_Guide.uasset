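; BP_Guide is a Forest level actor whose static mesh bobs up and down continuously.
; BeginPlay stores the mesh's starting relative Z height.
; Each Tick sets the relative Z to that height plus a degree-based sine of time since creation, scaled by BobSpeed and BobDistance.
; Only Z is supplied to the location update, so relative X and Y are left at the pin defaults.
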(event `self.ReceiveBeginPlay`
  (set `self.starting location` (.z (.location (`SceneComponent.GetRelativeTransform` (`self.StaticMesh`))))))

(event `self.ReceiveTick`
  (params (DeltaSeconds :type "Float (single-precision)"))
  (`SceneComponent.K2_SetRelativeLocation` (`self.StaticMesh`) (`KismetMathLibrary.MakeVector` 0.0 0.0 (+ (`self.starting location`) (* (`KismetMathLibrary.DegSin` (* (`self.GetGameTimeSinceCreation`) (`self.bob speed`))) (`self.bob distance`)))) false false))

(fn `UserConstructionScript`)