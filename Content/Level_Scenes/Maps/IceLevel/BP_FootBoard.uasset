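; BP_FootBoard is a vanishing, respawning platform in the ice level.
; When something overlaps its box while active, it lights up through a dynamic material and a timeline animates its opacity.
; After a short delay it spawns a hidden, non-colliding replacement at its original transform and destroys itself.
; Each new board's BeginPlay waits briefly, then SetParameters makes it active, visible and solid.
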(event `self.ReceiveBeginPlay`
  (set `self.active?` false)
  (bind _returnvalue (`PrimitiveComponent.CreateDynamicMaterialInstance` (`self.Cube`) 0 "/Game/Unreal_Asset/StarterContent/Materials/M_Bright.M_Bright" "None"))
  (bind _output_get (set `self.Dynamic` _returnvalue))
  (`MaterialInstanceDynamic.SetScalarParameterValue` _output_get "Bright" 0.0)
  (`MaterialInstanceDynamic.SetScalarParameterValue` _output_get "Opacity" 1.0)
  (set `self.SpawnTransform` (`self.GetTransform`))
  (`KismetSystemLibrary.Delay` 2.0)
  (`self.SetParameters`))

(event `self.Box.OnComponentBeginOverlap`
  (params (OverlappedComponent :type "PrimitiveComponent Object Reference") (OtherActor :type "Actor Object Reference") (OtherComp :type "PrimitiveComponent Object Reference") (OtherBodyIndex :type Integer) (bFromSweep :type Boolean) (SweepResult :type "HitResult Structure (by ref)"))
  (if (`self.active?`)
    (`MaterialInstanceDynamic.SetScalarParameterValue` (`self.Dynamic`) "Bright" 10.0)
    (`|ExecutionSequence`
      (:`then_0`
        (bind (_direction _alphachange) (`Timeline|Alpha`)
          (:`Update`
            (`MaterialInstanceDynamic.SetScalarParameterValue` (`self.Dynamic`) "Opacity" _alphachange))))
      (:`then_1`
        (`KismetSystemLibrary.Delay` 1.0)
        (bind _returnvalue (`|SpawnActorFromClass` "BP_FootBoard_C" (`self.SpawnTransform`) "Undefined" "MultiplyWithRoot" null null))
        (set `/Game/Level_Scenes/Maps/IceLevel/BP_FootBoard.active?` false _returnvalue)
        (bind _cube (`/Game/Level_Scenes/Maps/IceLevel/BP_FootBoard.Cube` _returnvalue))
        (`PrimitiveComponent.SetCollisionEnabled` _cube "NoCollision")
        (`SceneComponent.SetVisibility` _cube false false)
        (`self.K2_DestroyActor`)))))

(event `self.Box.OnComponentEndOverlap`
  (params (OverlappedComponent :type "PrimitiveComponent Object Reference") (OtherActor :type "Actor Object Reference") (OtherComp :type "PrimitiveComponent Object Reference") (OtherBodyIndex :type Integer)))

(fn `SetParameters`
  (bind _cube (`self.Cube`))
  (set `self.active?` true)
  (`PrimitiveComponent.SetCollisionEnabled` _cube "QueryAndPhysics")
  (`SceneComponent.SetVisibility` _cube true false))

(fn `UserConstructionScript`)